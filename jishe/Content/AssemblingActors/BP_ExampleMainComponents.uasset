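; Example actor in AssemblingActors that sets up lookup maps for its box and static mesh components, apparently as a template for assembly parts.
; Custom events map each box to a type value in EnumMap and to its mesh in MeshMap; an author note flags MakeEnumMap as consistently erroring.
; ReturnOriginLook is a placeholder material reset handling only StaticMesh1, with no material chosen.
; Nothing in this graph calls these events.
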(event EventBeginPlay)

(event Collision|EventActorBeginOverlap
  (params (OtherActor :type Actor%20Object%20Reference)))

(event EventTick
  (params (DeltaSeconds :type Float%20%28single-precision%29)))

(event EventMakeMeshMap
  (Variables|Default|SetMeshMap (Utilities|Map|MakeMap (Variables|Default|GetBox1) (Variables|Default|GetStaticMesh1) (Variables|Default|GetBox) (Variables|Default|GetStaticMesh2))))

(event EventMakeEnumMap
  (Variables|Default|SetEnumMap (Utilities|Map|MakeMap (Variables|Default|GetBox1) "Type1" (Variables|Default|GetBox) "Type2")))

(event EventReturnOriginLook
  (params (MeshComponents :type Scene%20Component%20Object%20Reference))
  (if (== MeshComponents (Variables|Default|GetStaticMesh1))
    ;[1 1 1] 选择自己的材质，其他的跟这一样
    (Rendering|Material|SetMaterial (Variables|Default|GetStaticMesh1) 0 0)))

(fn ConstructionScript)