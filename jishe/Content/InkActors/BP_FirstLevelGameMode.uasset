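; Game mode for the first level that connects the player pawn to the level's ink factory at startup.
; On BeginPlay it finds BP_InkFactory and, if valid, passes it to the player pawn through SetInkActorFactoryMessage.
; It then caches the location and box extent of the Wood actor.
; GetBoxExtent exposes the cached extent but returns a zero vector for location instead of the cached one.
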(event EventBeginPlay
  (bind _returnvalue (Actor|GetActorOfClass "/Game/InkActors/BP_InkFactory.BP_InkFactory_C"))
  (Utilities|IsValid _returnvalue
    (:Is%20Valid
      (Class|BPIControllerInerfaceLevel1|SetInkActorFactory(Message) (Game|Player|GetPlayerPawn 0) _returnvalue)
      (bind _returnvalue_2 (Actor|GetActorOfClass "/Script/jishe.Wood"))
      (Variables|Default|SetLocation (Transformation|GetActorLocation _returnvalue_2))
      (Variables|Default|SetBox%20Extent (Variables|/Script/Engine.BoxComponent|GetBoxExtent (Variables|/Script/jishe.Wood|GetBox _returnvalue_2))))))

(fn ConstructionScript)

(fn GetBoxExtent
  (return (Variables|Default|GetBox%20Extent) "0, 0, 0"))