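; BP_InkLine is an ink-line actor built around a static mesh, with its appearance driven by external calls.
; Its custom events toggle the mesh's visibility and swap slot 0 to a supplied examination material.
; An unconnected chain would create a dynamic Positionselect material from the GameMode's box location and halved extents, but it never runs.
; BeginPlay and the construction script are empty.
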(event EventBeginPlay)

(event EventChangeMaterialtoExamination
  (params (Instance :type Material%20Instance%20Object%20Reference))
  (Rendering|Material|SetMaterial (Variables|Default|GetStaticMesh) 0 Instance))

(event EventSetStaticMeshVisibility
  (params (Visibility :type Boolean))
  (Rendering|SetVisibility (Variables|Default|GetStaticMesh) Visibility false))

(fn ConstructionScript)