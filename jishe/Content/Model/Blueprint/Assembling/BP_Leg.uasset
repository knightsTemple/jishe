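; BP_Leg is the leg part in an assembling system, defining what it connects to through data maps.
; MakeEnumMap assigns every connection key (long piece, desk, fan and hold joints) the same type, Type1.
; MakeMeshMap pairs the same keys with their corresponding mesh components or assets.
; ReturnOriginLook is an empty stub, and the construction script and standard events contain no logic.
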(event EventBeginPlay)

(event Collision|EventActorBeginOverlap
  (params (OtherActor :type Actor%20Object%20Reference)))

(event EventTick
  (params (DeltaSeconds :type Float%20%28single-precision%29)))

(event EventMakeMeshMap
  (Variables|Default|SetMeshMap (Utilities|Map|MakeMap (Variables|Default|GetLegAndLong) (Variables|Default|GetUpperLong) (Variables|Default|GetLongAndDesk) (Variables|Default|GetDeskLeg) (Variables|Default|GetDeskConnection) (Variables|Default|GetDeskConnect) (Variables|Default|GetLongAndFan) (Variables|Default|GetByFan) (Variables|Default|GetFanAndHold) (Variables|Default|GetFanHold) (Variables|Default|GetFanAndHold2) (Variables|Default|GetFanHold_2))))

(event EventMakeEnumMap
  (Variables|Default|SetEnumMap (Utilities|Map|MakeMap (Variables|Default|GetLegAndLong) "Type1" (Variables|Default|GetLongAndDesk) "Type1" (Variables|Default|GetDeskConnection) "Type1" (Variables|Default|GetLongAndFan) "Type1" (Variables|Default|GetFanAndHold) "Type1" (Variables|Default|GetFanAndHold2) "Type1")))

(event EventReturnOriginLook
  (params (MeshComponents :type Scene%20Component%20Object%20Reference)))

(fn ConstructionScript)