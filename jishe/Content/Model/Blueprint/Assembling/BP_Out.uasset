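; BP_Out is an assembling model actor for an outlet assembly of six parts, including wheat outlets, out boards and other outlets.
; MakeMeshMap links each part key to its mesh component, and MakeEnumMap links the same keys to type values.
; ReturnOriginLook resets the passed mesh's first material to MI_Wood, using a component comparison chain with a primitive-component cast as fallback.
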(event EventBeginPlay)

(event Collision|EventActorBeginOverlap
  (params (OtherActor :type Actor%20Object%20Reference)))

(event EventTick
  (params (DeltaSeconds :type Float%20%28single-precision%29)))

(event EventMakeEnumMap
  (Variables|Default|SetEnumMap (Utilities|Map|MakeMap (Variables|Default|GetF0_WheatOut) "Type1" (Variables|Default|GetF1_OutBoardBack) "Type2" (Variables|Default|GetF2_OutBoardFront) "Type3" (Variables|Default|GetF3_WheatOutUp) "Type4" (Variables|Default|GetF4_OtherOut) "Type5" (Variables|Default|GetF5_OtherUp) "Type6")))

(event EventMakeMeshMap
  (Variables|Default|SetMeshMap (Utilities|Map|MakeMap (Variables|Default|GetF0_WheatOut) (Variables|Default|GetC0_Out) (Variables|Default|GetF1_OutBoardBack) (Variables|Default|GetC1_OutBoardBack) (Variables|Default|GetF2_OutBoardFront) (Variables|Default|GetC2_OutBoardFront) (Variables|Default|GetF3_WheatOutUp) (Variables|Default|GetC3_WheatOutUp) (Variables|Default|GetF4_OtherOut) (Variables|Default|GetC4_OtherOut) (Variables|Default|GetF5_OtherUp) (Variables|Default|GetC5_OtherUp))))

(event EventReturnOriginLook
  (params (MeshComponents :type Scene%20Component%20Object%20Reference))
  (if (== MeshComponents (Variables|Default|GetC0_Out))
    (Rendering|Material|SetMaterial (Variables|Default|GetC0_Out) 0 "/Game/Fab/Megascans/Surfaces/Plywood_vf1oairg/Medium/MI_Wood.MI_Wood")
    (elif (== MeshComponents (Variables|Default|GetC1_OutBoardBack))
      (Rendering|Material|SetMaterial (Variables|Default|GetC1_OutBoardBack) 0 "/Game/Fab/Megascans/Surfaces/Plywood_vf1oairg/Medium/MI_Wood.MI_Wood")
      (elif (== MeshComponents (Variables|Default|GetC2_OutBoardFront))
        (Rendering|Material|SetMaterial (Variables|Default|GetC2_OutBoardFront) 0 "/Game/Fab/Megascans/Surfaces/Plywood_vf1oairg/Medium/MI_Wood.MI_Wood")
        (elif (== MeshComponents (Variables|Default|GetC3_WheatOutUp))
          (Rendering|Material|SetMaterial (Variables|Default|GetC3_WheatOutUp) 0 "/Game/Fab/Megascans/Surfaces/Plywood_vf1oairg/Medium/MI_Wood.MI_Wood")
          (elif (== MeshComponents (Variables|Default|GetC4_OtherOut))
            (Rendering|Material|SetMaterial (Variables|Default|GetC4_OtherOut) 0 "/Game/Fab/Megascans/Surfaces/Plywood_vf1oairg/Medium/MI_Wood.MI_Wood")
            (elif (== MeshComponents (Variables|Default|GetC5_OtherUp))
              (Rendering|Material|SetMaterial (Variables|Default|GetC5_OtherUp) 0 "/Game/Fab/Megascans/Surfaces/Plywood_vf1oairg/Medium/MI_Wood.MI_Wood")
              (else
                (bind _as基元组件 (Utilities|Casting|CastToPrimitiveComponent MeshComponents))
                (Rendering|Material|SetMaterial _as基元组件 0 "/Game/Fab/Megascans/Surfaces/Plywood_vf1oairg/Medium/MI_Wood.MI_Wood")))))))))

(fn ConstructionScript)