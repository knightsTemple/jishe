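; BP_Some is an assembling-model actor with four mesh parts: wheat out, back and front outboards, and wheat out up.
; MakeEnumMap maps the F-prefixed part keys to type values, and MakeMeshMap maps the same keys to their C-prefixed mesh components.
; ReturnOriginLook compares a given component against each part and resets the match's first material slot to the shared MI_vf1oairg material.
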(event EventBeginPlay)

(event Collision|EventActorBeginOverlap
  (params (OtherActor :type Actor%20Object%20Reference)))

(event EventTick
  (params (DeltaSeconds :type Float%20%28single-precision%29)))

(event EventMakeEnumMap
  (Variables|Default|SetEnumMap (Utilities|Map|MakeMap (Variables|Default|GetF0_WheatOut) "Type1" (Variables|Default|GetF1_OutBoardBack) "Type2" (Variables|Default|GetF2_OutBoardFront) "Type3" (Variables|Default|GetF3_WheatOutUp) "Type4")))

(event EventMakeMeshMap
  (Variables|Default|SetMeshMap (Utilities|Map|MakeMap (Variables|Default|GetF0_WheatOut) (Variables|Default|GetC0_Out) (Variables|Default|GetF1_OutBoardBack) (Variables|Default|GetC1_OutBoardBack) (Variables|Default|GetF2_OutBoardFront) (Variables|Default|GetC2_OutBoardFront) (Variables|Default|GetF3_WheatOutUp) (Variables|Default|GetC3_WheatOutUp))))

(event EventReturnOriginLook
  (params (MeshComponents :type Scene%20Component%20Object%20Reference))
  (if (== MeshComponents (Variables|Default|GetC0_Out))
    (Rendering|Material|SetMaterial (Variables|Default|GetC0_Out) 0 "/Game/Fab/Megascans/Surfaces/Plywood_vf1oairg/Medium/MI_vf1oairg.MI_vf1oairg")
    (elif (== MeshComponents (Variables|Default|GetC1_OutBoardBack))
      (Rendering|Material|SetMaterial (Variables|Default|GetC1_OutBoardBack) 0 "/Game/Fab/Megascans/Surfaces/Plywood_vf1oairg/Medium/MI_vf1oairg.MI_vf1oairg")
      (elif (== MeshComponents (Variables|Default|GetC2_OutBoardFront))
        (Rendering|Material|SetMaterial (Variables|Default|GetC2_OutBoardFront) 0 "/Game/Fab/Megascans/Surfaces/Plywood_vf1oairg/Medium/MI_vf1oairg.MI_vf1oairg")
        (elif (== MeshComponents (Variables|Default|GetC3_WheatOutUp))
          (Rendering|Material|SetMaterial (Variables|Default|GetC3_WheatOutUp) 0 "/Game/Fab/Megascans/Surfaces/Plywood_vf1oairg/Medium/MI_vf1oairg.MI_vf1oairg"))))))

(fn ConstructionScript)