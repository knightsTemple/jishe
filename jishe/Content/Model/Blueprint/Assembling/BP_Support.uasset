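; BP_Support is an assembly actor for a support structure built from nine parts, including legs, connectors, desk pieces and fan holders.
; MakeEnumMap and MakeMeshMap key each F-prefixed assembly slot to its type value and its mesh component.
; ReturnOriginLook compares the passed component against each part through a branch chain and restores the shared original material on the match.
; BeginPlay, Tick and the construction script are empty.
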(event EventBeginPlay)

(event Collision|EventActorBeginOverlap
  (params (OtherActor :type Actor%20Object%20Reference)))

(event EventTick
  (params (DeltaSeconds :type Float%20%28single-precision%29)))

(event EventMakeMeshMap
  (Variables|Default|SetMeshMap (Utilities|Map|MakeMap (Variables|Default|GetF0_PlaceLeg) (Variables|Default|GetC0_Leg1) (Variables|Default|GetF1_ShortConnect) (Variables|Default|GetC1_ShortConnect) (Variables|Default|GetF2_LongConnect) (Variables|Default|GetC2_LongConnect1) (Variables|Default|GetF3_LegAndLong) (Variables|Default|GetC3_Long) (Variables|Default|GetF4_LongAndDesk) (Variables|Default|GetC4_DeskLeg) (Variables|Default|GetF5_DeskConnection) (Variables|Default|GetC5_DeskConnect) (Variables|Default|GetF6_LongAndFan) (Variables|Default|GetC6_ByFan) (Variables|Default|GetF7_FanAndHold2) (Variables|Default|GetC7_FanHold_2) (Variables|Default|GetF8_FanAndHold) (Variables|Default|GetC8_FanHold))))

(event EventMakeEnumMap
  (Variables|Default|SetEnumMap (Utilities|Map|MakeMap (Variables|Default|GetF0_PlaceLeg) "Type1" (Variables|Default|GetF1_ShortConnect) "Type2" (Variables|Default|GetF2_LongConnect) "Type3" (Variables|Default|GetF3_LegAndLong) "Type4" (Variables|Default|GetF4_LongAndDesk) "Type5" (Variables|Default|GetF5_DeskConnection) "Type6" (Variables|Default|GetF6_LongAndFan) "Type7" (Variables|Default|GetF7_FanAndHold2) "Type8" (Variables|Default|GetF8_FanAndHold) "Type9")))

(event EventReturnOriginLook
  (params (MeshComponents :type Scene%20Component%20Object%20Reference))
  (if (== MeshComponents (Variables|Default|GetC0_Leg1))
    (Rendering|Material|SetMaterial (Variables|Default|GetC0_Leg1) 0 "/Game/Fab/Megascans/Surfaces/Plywood_vf1oairg/Medium/MI_vf1oairg.MI_vf1oairg")
    (elif (== MeshComponents (Variables|Default|GetC1_ShortConnect))
      (Rendering|Material|SetMaterial (Variables|Default|GetC1_ShortConnect) 0 "/Game/Fab/Megascans/Surfaces/Plywood_vf1oairg/Medium/MI_vf1oairg.MI_vf1oairg")
      (elif (== MeshComponents (Variables|Default|GetC2_LongConnect1))
        (Rendering|Material|SetMaterial (Variables|Default|GetC2_LongConnect1) 0 "/Game/Fab/Megascans/Surfaces/Plywood_vf1oairg/Medium/MI_vf1oairg.MI_vf1oairg")
        (elif (== MeshComponents (Variables|Default|GetC3_Long))
          (Rendering|Material|SetMaterial (Variables|Default|GetC3_Long) 0 "/Game/Fab/Megascans/Surfaces/Plywood_vf1oairg/Medium/MI_vf1oairg.MI_vf1oairg")
          (elif (== MeshComponents (Variables|Default|GetC4_DeskLeg))
            (Rendering|Material|SetMaterial (Variables|Default|GetC4_DeskLeg) 0 "/Game/Fab/Megascans/Surfaces/Plywood_vf1oairg/Medium/MI_vf1oairg.MI_vf1oairg")
            (elif (== MeshComponents (Variables|Default|GetC5_DeskConnect))
              (Rendering|Material|SetMaterial (Variables|Default|GetC5_DeskConnect) 0 "/Game/Fab/Megascans/Surfaces/Plywood_vf1oairg/Medium/MI_vf1oairg.MI_vf1oairg")
              (elif (== MeshComponents (Variables|Default|GetC6_ByFan))
                (Rendering|Material|SetMaterial (Variables|Default|GetC6_ByFan) 0 "/Game/Fab/Megascans/Surfaces/Plywood_vf1oairg/Medium/MI_vf1oairg.MI_vf1oairg")
                (elif (== MeshComponents (Variables|Default|GetC7_FanHold_2))
                  (Rendering|Material|SetMaterial (Variables|Default|GetC7_FanHold_2) 0 "/Game/Fab/Megascans/Surfaces/Plywood_vf1oairg/Medium/MI_vf1oairg.MI_vf1oairg")
                  (elif (== MeshComponents (Variables|Default|GetC8_FanHold))
                    (Rendering|Material|SetMaterial (Variables|Default|GetC8_FanHold) 0 "/Game/Fab/Megascans/Surfaces/Plywood_vf1oairg/Medium/MI_vf1oairg.MI_vf1oairg")))))))))))

(fn ConstructionScript)