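; BP_WheatIn is a wheat-inlet model for assembling, made of ten mesh parts such as an axis, adjusters, blocks and inlet pieces.
; MakeEnumMap maps each F-prefixed part key to a type, and MakeMeshMap maps the same keys to mesh components.
; ReturnOriginLook restores a given component's original material through a branch chain.
; An author note flags a recurring, unexplained error at MakeEnumMap.
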(event EventBeginPlay)

(event Collision|EventActorBeginOverlap
  (params (OtherActor :type Actor%20Object%20Reference)))

(event EventTick
  (params (DeltaSeconds :type Float%20%28single-precision%29)))

(event EventMakeMeshMap
  (Variables|Default|SetMeshMap (Utilities|Map|MakeMap (Variables|Default|GetF0_Axis) (Variables|Default|GetC0_Axis) (Variables|Default|GetF1_Block1) (Variables|Default|GetC1_AdjustHand) (Variables|Default|GetF2_AdjustStick) (Variables|Default|GetC2_AdjustStick) (Variables|Default|GetF3_AdjustSquare) (Variables|Default|GetC3_AdjustSquare) (Variables|Default|GetF4_BlockFront) (Variables|Default|GetC4_BlockFront) (Variables|Default|GetF5_BlockBack) (Variables|Default|GetC5_BlockBack) (Variables|Default|GetF6_WheatIn) (Variables|Default|GetC6_WheatInBack) (Variables|Default|GetF7_WheatIn) (Variables|Default|GetC7_WheatInRight) (Variables|Default|GetF8_WheatIn) (Variables|Default|GetC8_WheatInLeft) (Variables|Default|GetF9_WheatIn) (Variables|Default|GetC9_WheatInFront))))

(event EventMakeEnumMap
  (Variables|Default|SetEnumMap (Utilities|Map|MakeMap (Variables|Default|GetF0_Axis) "Type1" (Variables|Default|GetF1_Block1) "Type2" (Variables|Default|GetF2_AdjustStick) "Type3" (Variables|Default|GetF3_AdjustSquare) "Type4" (Variables|Default|GetF4_BlockFront) "Type5" (Variables|Default|GetF5_BlockBack) "Type6" (Variables|Default|GetF6_WheatIn) "Type7" (Variables|Default|GetF7_WheatIn) "Type8" (Variables|Default|GetF8_WheatIn) "Type9" (Variables|Default|GetF9_WheatIn) "Type10")))

(event EventReturnOriginLook
  (params (MeshComponents :type Scene%20Component%20Object%20Reference))
  (if (== MeshComponents (Variables|Default|GetC0_Axis))
    (Rendering|Material|SetMaterial (Variables|Default|GetC0_Axis) 0 "/Game/Fab/Megascans/Surfaces/Plywood_vf1oairg/Medium/MI_vf1oairg.MI_vf1oairg")
    (elif (== MeshComponents (Variables|Default|GetC1_AdjustHand))
      (Rendering|Material|SetMaterial (Variables|Default|GetC1_AdjustHand) 0 "/Game/Fab/Megascans/Surfaces/Plywood_vf1oairg/Medium/MI_vf1oairg.MI_vf1oairg")
      (elif (== MeshComponents (Variables|Default|GetC2_AdjustStick))
        (Rendering|Material|SetMaterial (Variables|Default|GetC2_AdjustStick) 0 "/Game/Fab/Megascans/Surfaces/Plywood_vf1oairg/Medium/MI_vf1oairg.MI_vf1oairg")
        (elif (== MeshComponents (Variables|Default|GetC3_AdjustSquare))
          (Rendering|Material|SetMaterial (Variables|Default|GetC3_AdjustSquare) 0 "/Game/Fab/Megascans/Surfaces/Plywood_vf1oairg/Medium/MI_vf1oairg.MI_vf1oairg")
          (elif (== MeshComponents (Variables|Default|GetC4_BlockFront))
            (Rendering|Material|SetMaterial (Variables|Default|GetC4_BlockFront) 0 "/Game/Fab/Megascans/Surfaces/Plywood_vf1oairg/Medium/MI_vf1oairg.MI_vf1oairg")
            (elif (== MeshComponents (Variables|Default|GetC5_BlockBack))
              (Rendering|Material|SetMaterial (Variables|Default|GetC5_BlockBack) 0 "/Game/Fab/Megascans/Surfaces/Plywood_vf1oairg/Medium/MI_vf1oairg.MI_vf1oairg")
              (elif (== MeshComponents (Variables|Default|GetC6_WheatInBack))
                (Rendering|Material|SetMaterial (Variables|Default|GetC6_WheatInBack) 0 "/Game/Fab/Megascans/Surfaces/Plywood_vf1oairg/Medium/MI_vf1oairg.MI_vf1oairg")
                (elif (== MeshComponents (Variables|Default|GetC7_WheatInRight))
                  (Rendering|Material|SetMaterial (Variables|Default|GetC7_WheatInRight) 0 "/Game/Fab/Megascans/Surfaces/Plywood_vf1oairg/Medium/MI_vf1oairg.MI_vf1oairg")
                  (elif (== MeshComponents (Variables|Default|GetC8_WheatInLeft))
                    (Rendering|Material|SetMaterial (Variables|Default|GetC8_WheatInLeft) 0 "/Game/Fab/Megascans/Surfaces/Plywood_vf1oairg/Medium/MI_vf1oairg.MI_vf1oairg")
                    (elif (== MeshComponents (Variables|Default|GetC9_WheatInFront))
                      (Rendering|Material|SetMaterial (Variables|Default|GetC9_WheatInFront) 0 "/Game/Fab/Megascans/Surfaces/Plywood_vf1oairg/Medium/MI_vf1oairg.MI_vf1oairg"))))))))))))

(fn ConstructionScript)